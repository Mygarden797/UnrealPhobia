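; BP_MyProtoPlayer is a player Blueprint for the network prototype that handles inventory input and shows a crosshair.
; Enhanced Input actions for slot selection, drop-off and pick-up forward straight to TriggerInventory, with the slot value truncated to an integer.
; BeginPlay creates WBP_Crosshair and adds it to the viewport without a local-control check.
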(event `EnhancedInput|/Game/ThirdPerson/Input/Actions/IA_SelectSlot`
  (params (ActionValue :type "Float (double-precision)") (ElapsedSeconds :type "Float (double-precision)") (TriggeredSeconds :type "Float (double-precision)") (InputAction :type "InputAction Object Reference" :default "/Game/ThirdPerson/Input/Actions/IA_SelectSlot.IA_SelectSlot"))
  (:`Started`
    (`TriggerInventory.SelectSlot` (`self.TriggerInventory`) (`KismetMathLibrary.FTrunc` ActionValue))))

(event `EnhancedInput|/Game/ThirdPerson/Input/Actions/IA_DropOff`
  (params (ActionValue :type Boolean) (ElapsedSeconds :type "Float (double-precision)") (TriggeredSeconds :type "Float (double-precision)") (InputAction :type "InputAction Object Reference" :default "/Game/ThirdPerson/Input/Actions/IA_DropOff.IA_DropOff"))
  (:`Started`
    (`TriggerInventory.DropOff` (`self.TriggerInventory`))))

(event `EnhancedInput|/Game/ThirdPerson/Input/Actions/IA_PickUp`
  (params (ActionValue :type Boolean) (ElapsedSeconds :type "Float (double-precision)") (TriggeredSeconds :type "Float (double-precision)") (InputAction :type "InputAction Object Reference" :default "/Game/ThirdPerson/Input/Actions/IA_PickUp.IA_PickUp"))
  (:`Started`
    (`TriggerInventory.PickUp` (`self.TriggerInventory`))))

(event `self.ReceiveBeginPlay`
  (bind _returnvalue (`|CreateWidget` "/Game/UI/WBP_Crosshair.WBP_Crosshair_C"))
  (`UserWidget.AddToViewport` _returnvalue 0))

(fn `UserConstructionScript`)